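; DragableObject is an unfinished interactable Blueprint meant to let the player drag an object with the cursor.
; Clicking the object opens a gate, and releasing it or moving the cursor off closes it.
; The gate's exit calls DragObject, but its entry and the input toggle sit in unconnected nodes.
; DragObject is empty, with only disconnected draft nodes for a Y-axis move and debug print.
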(event OnClicked(Object)
  (params (TouchedActor :type Actor%20Object%20Reference) (ButtonPressed :type Key%20Structure))
  ;[1 1 1] Object Clicked
  (Utilities|FlowControl|Gate true) ; enters at Open
)

(event OnReleased(Object)
  (params (TouchedActor :type Actor%20Object%20Reference) (ButtonReleased :type Key%20Structure))
  ;[1 1 1] Object Clicked
  (Utilities|FlowControl|Gate true) ; enters at Close
)

(event OnEndCursorOver(Object)
  (params (TouchedActor :type Actor%20Object%20Reference))
  ;[1 1 1] Object Clicked
  (Utilities|FlowControl|Gate true) ; enters at Close
)

(event EventTick
  (params (DeltaSeconds :type Float%20%28single-precision%29)))

(fn ConstructionScript)

(fn DragObject)