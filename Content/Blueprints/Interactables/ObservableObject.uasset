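; Clickable interactable that moves the player's view to a close-up of itself for observation.
; Hovering reveals the collision box while the player is not observing; clicking blends the view target to this actor and adds a ReturnToBaseCamera_UI widget.
; The click also sets IsObserving on PlayerCamera_Pawn and disables the box's collision.
; Tick polls that flag to restore query-only collision once observing ends.
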(event OnClicked(CollisionBox)
  (params (TouchedComponent :type Primitive%20Component%20Object%20Reference) (ButtonPressed :type Key%20Structure))
  (bind _asplayer_camera_pawn (Utilities|Casting|CastToPlayerCamera_Pawn (Game|Player|GetPlayerPawn 0)))
  (if (Variables|/Game/Blueprints/PlayerCamera_Pawn.PlayerCamera_Pawn_C|GetIsObserving _asplayer_camera_pawn)
    (Collision|SetCollisionEnabled (Variables|Default|GetCollisionBox) "QueryOnly")
    (else
      (Variables|Default|SetCameraInMotion true)
      (Game|Player|SetViewTargetwithBlend (Game|GetPlayerController 0) self 0.5 "VTBlend_Cubic" 0.0 false)
      (Variables|Default|SetCameraAtLocation true)
      (bind _returnvalue (UserInterface|CreateWidget "/Game/Widgets/ReturnToBaseCamera_UI.ReturnToBaseCamera_UI_C"))
      (UserInterface|Viewport|AddtoViewport _returnvalue 1)
      (bind _asplayer_camera_pawn_2 (Utilities|Casting|CastToPlayerCamera_Pawn (Game|Player|GetPlayerPawn 0)))
      (Variables|/Game/Blueprints/PlayerCamera_Pawn.PlayerCamera_Pawn_C|SetIsObserving _asplayer_camera_pawn_2 true)
      (Development|PrintString "Observing")
      (Collision|SetCollisionEnabled (Variables|Default|GetCollisionBox) "NoCollision"))))

(event MouseInput|EventActorBeginCursorOver
  (bind _asplayer_camera_pawn (Utilities|Casting|CastToPlayerCamera_Pawn (Game|Player|GetPlayerPawn 0)))
  (if (not (Variables|/Game/Blueprints/PlayerCamera_Pawn.PlayerCamera_Pawn_C|GetIsObserving _asplayer_camera_pawn))
    (Rendering|SetVisibility (Variables|Default|GetCollisionBox) true true)))

(event MouseInput|EventActorEndCursorOver
  (Rendering|SetVisibility (Variables|Default|GetCollisionBox) false true))

(event EventBeginPlay
  (Rendering|SetVisibility (Variables|Default|GetCollisionBox) false false))

(event EventTick
  (params (DeltaSeconds :type Float%20%28single-precision%29))
  (bind _asplayer_camera_pawn (Utilities|Casting|CastToPlayerCamera_Pawn (Game|Player|GetPlayerPawn 0)))
  (if (not (Variables|/Game/Blueprints/PlayerCamera_Pawn.PlayerCamera_Pawn_C|GetIsObserving _asplayer_camera_pawn))
    (Collision|SetCollisionEnabled (Variables|Default|GetCollisionBox) "QueryOnly")))

(fn ConstructionScript)